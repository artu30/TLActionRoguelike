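; BP_Cannon is an AI turret actor that tracks the player and fires magic projectiles at them.
; Every tick it rotates to face the player character using a look-at rotation.
; A looping timer started on BeginPlay spawns a BP_MagicProjectile_AI from its location and rotation every couple of seconds, owned by the cannon and always spawned regardless of collision.
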(event `self.ReceiveBeginPlay`
  (`KismetSystemLibrary.K2_SetTimerDelegate` (delegate `SpawnProjectile`) 2.0 true))

(event `SpawnProjectile`
  (`|SpawnActorFromClass` "/Game/TLActionRoguelike/Projectiles/BP_MagicProjectile_AI.BP_MagicProjectile_AI_C" (`KismetMathLibrary.MakeTransform` (`self.K2_GetActorLocation`) (`self.K2_GetActorRotation`)) "AlwaysSpawn" "MultiplyWithRoot" self null))

(event `self.ReceiveTick`
  (params (DeltaSeconds :type "Float (single-precision)"))
  (`self.K2_SetActorRotation` (`KismetMathLibrary.FindLookAtRotation` (`self.K2_GetActorLocation`) (`self.K2_GetActorLocation` (`self.PlayerCharacter`)))))

(fn `UserConstructionScript`)