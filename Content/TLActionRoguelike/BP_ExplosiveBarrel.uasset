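; Explosive barrel actor that detonates on a fixed timer a few seconds after BeginPlay.
; The server alone starts the timer, then calls a multicast that fires the radial force impulse, hides the barrel and disables its collision on all machines.
; A short lifespan set after the blast delays destruction instead of destroying the actor immediately.
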(event `self.ReceiveBeginPlay`
  ;[1 1 1] Same
  (`/Engine/EditorBlueprintResources/ActorMacros.Switch Has Authority`
    (:`Authority`
      (`KismetSystemLibrary.K2_SetTimerDelegate` (delegate `ExplodeEvent`) 4.0))))

(event `ExplodeEvent`
  (`self.MulticastExplode`)
  (`self.SetLifeSpan` 2.0))

(event `MulticastExplode`
  (`RadialForceComponent.FireImpulse` (`self.RadialForceComp`))
  (`self.SetActorHiddenInGame` true)
  (`self.SetActorEnableCollision` false))

(fn `UserConstructionScript`)